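; Base actor for buildable pieces that preview in front of the camera, then self-destruct once placed if ground support is too low.
; The preview traces to GroundSurface height, then snaps SnapNodes to nearby nodes with matching structure, piece and snap IDs.
; Placing switches mesh collision profiles and starts a per-tick stability check estimating base coverage from overlapping grounds' bounds.
; Child classes override SetPlacementBase; Data assignment in Initialize is disconnected for testing.
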(event `self.ReceiveTick`
  (params (DeltaSeconds :type "Float (single-precision)"))
  (if (`self.Placed`)
    (bind _stability_percent (`self.Stability Check`))
    (if (not (> _stability_percent (`self.Stability Threshold`)))
      (`self.K2_DestroyActor`))
    (else
      (`self.PlacePreview`))))

(fn `Check Snap Legality`
  (params (`Node 1` :type "/Game/Blueprints/SnapNode Object Reference") (`Node 2` :type "/Game/Blueprints/SnapNode Object Reference"))
  (returns (Return :type Boolean))
  (locals (Placeable :type "/Game/Blueprints/Placeable Object Reference") (Node2 :type "/Game/Blueprints/SnapNode Object Reference") (Node :type "/Game/Blueprints/SnapNode Object Reference") (NewLocalVar :type "/Game/Blueprints/SnapNode Object Reference"))
  (bind _node2 (`local.Node2`))
  (bind (_seekingid_structurenum _seekingid_piecenum) (break `/Game/StructsAndEnums/PieceID` (`/Game/Blueprints/SnapNode.SeekingID` _node2)))
  (set `local.Node` `Node 1`)
  (set `local.Node2` `Node 2`)
  (bind _asplaceable (cast `/Game/Blueprints/Placeable` (`self.GetParentActor` `Node 1`))
    (:`then`
      (set `local.Placeable` _asplaceable)
      (bind (_id_structurenum _id_piecenum) (break `/Game/StructsAndEnums/PieceID` (`/Game/Blueprints/Primary_Placeable.ID` (`/Game/Blueprints/Placeable.Data` _asplaceable))))
      (if (and (== _id_structurenum _seekingid_structurenum) (== _id_piecenum _seekingid_piecenum) (== (`/Game/Blueprints/SnapNode.SeekingSnapID` _node2) (`/Game/Blueprints/SnapNode.SnapID` (`local.Node`))))
        (return true)
        (else
          (return false))))
    (:`CastFailed`
      (`KismetSystemLibrary.PrintString` "Cast failed, that's bad"))))

(fn `GetPlaceLocation`
  (returns (Location :type "Vector Structure"))
  (bind _camera (`self.Camera`))
  (return (+ (`SceneComponent.K2_GetComponentLocation` _camera) (* (`KismetMathLibrary.Normal` (`KismetMathLibrary.GetForwardVector` (`SceneComponent.K2_GetComponentRotation` _camera))) (`self.Distance`)))))

(fn `Initialize`
  (params (Camera :type "CameraComponent Object Reference") (Data :type "/Game/Blueprints/Primary_Placeable Object Reference"))
  (set `self.Camera` Camera)
  (`self.Set Placement Base`)
  (`self.Set Child Arrays`))

(fn `Move To Ground`
  (params (Obj :type "Object Object Reference"))
  (bind (_returnvalue_x _returnvalue_y) (`KismetMathLibrary.BreakVector` (`SceneComponent.K2_GetComponentLocation` (`self.Placement Base`))))
  (bind _asground_surface (cast `/Game/Blueprints/GroundSurface` Obj))
  (bind _location (`/Game/Blueprints/GroundSurface.Return Location` _asground_surface))
  (`self.K2_TeleportTo` (+ (`KismetMathLibrary.MakeVector` _returnvalue_x _returnvalue_y (.z _location)) (- (`SceneComponent.K2_GetComponentLocation` (`self.DefaultSceneRoot`)) (`SceneComponent.K2_GetComponentLocation` (`self.Placement Base`)))) (`self.Rotation`)))

(fn `Place`
  (set `self.Placed` true)
  (for _array_element (`self.K2_GetComponentsByClass` "/Script/Engine.MeshComponent")
    (`PrimitiveComponent.SetCollisionProfileName` _array_element "PlacedBlock" true)))

(fn `PlacePreview`
  (bind _returnvalue (`SceneComponent.K2_GetComponentLocation` (`self.Placement Base`)))
  (bind (_returnvalue_x _returnvalue_y _returnvalue_z) (`KismetMathLibrary.BreakVector` (`SceneComponent.K2_GetComponentLocation` (`self.Placement Base`))))
  ; Get Initial Location
  (bind _location (`self.GetPlaceLocation`))
  (`self.K2_TeleportTo` _location (`self.Rotation`))
  ; Cast for Ground Surface
  (bind (_outhit _returnvalue_2) (`KismetSystemLibrary.LineTraceSingle` (+ _returnvalue (0.0 0.0 50.0)) (- _returnvalue (0.0 0.0 200.0)) "TraceTypeQuery3" false (`self.Grounds`)))
  (if _returnvalue_2
    (`self.Move To Ground` (`.HitActor` (`GameplayStatics.BreakHitResult` _outhit)))
    ; Loop through snap nodes
    (for _array_element (`self.SnapNodes`) :!label _label
      (bind _succesful (`self.TryToSnap` _array_element))
      (if _succesful
        (return)))
    (else
      ; Try to Place Above Ground if Below It
      (if (< _returnvalue_z 0.0)
        (bind (_outhit_2 _returnvalue_3) (`KismetSystemLibrary.LineTraceSingle` (`SceneComponent.K2_GetComponentLocation` (`self.Placement Base`)) (`KismetMathLibrary.MakeVector` _returnvalue_x _returnvalue_y (+ _returnvalue_z (`self.Distance`))) "TraceTypeQuery3" false (`self.Grounds`)))
        (if _returnvalue_3
          (`self.Move To Ground` (`.HitActor` (`GameplayStatics.BreakHitResult` _outhit_2)))
          (goto _label)
          (else
            (goto _label)))))))

(fn `Rotate`
  (params (Dir :type "Float (double-precision)"))
  (set `self.Rotation` (`KismetMathLibrary.ComposeRotators` (`self.Rotation`) (`KismetMathLibrary.MakeRotator` 0.0 0.0 Dir))))

(fn `Set Child Arrays`
  (for _array_element (`self.GetAllChildActors` true)
    (bind _asbase_surface (cast `/Game/Blueprints/BaseSurface` _array_element)
      (:`then`
        (`KismetArrayLibrary.Array_Add` (`self.Bases`) _asbase_surface))
      (:`CastFailed`
        (bind _assnap_node (cast `/Game/Blueprints/SnapNode` _array_element)
          (:`then`
            (`KismetArrayLibrary.Array_Add` (`self.SnapNodes`) _assnap_node))
          (:`CastFailed`
            (bind _asground_surface (cast `/Game/Blueprints/GroundSurface` _array_element))
            (`KismetArrayLibrary.Array_Add` (`self.Grounds`) _asground_surface)))))))

(fn `Set Placement Base`
  (set `self.Placement Base` (`self.Base`)))

(fn `Stability Check`
  (returns (`Stability Percent` :type "Float (double-precision)"))
  (locals (CurrHeight :type "Float (double-precision)") (CurrWidth :type "Float (double-precision)") (`Total Surface` :type "Float (double-precision)") (`Covered Surface` :type "Float (double-precision)") (CurrBase :type "/Game/Blueprints/BaseSurface Object Reference") (CurrGround :type "/Game/Blueprints/GroundSurface Object Reference"))
  (bind _cube (`/Game/Blueprints/BaseSurface.Cube` (`local.CurrBase`)))
  (bind (_returnvalue_x _returnvalue_y) (`KismetMathLibrary.BreakVector` (`SceneComponent.K2_GetComponentLocation` _cube)))
  (bind (_returnvalue_x_2 _returnvalue_y_2) (`KismetMathLibrary.BreakVector` (* (`SceneComponent.K2_GetComponentScale` _cube) 0.5)))
  (bind _returnvalue (+ _returnvalue_x_2 _returnvalue_x))
  (bind _returnvalue_2 (+ _returnvalue_y_2 _returnvalue_y))
  (for _array_element (`self.Bases`)
    ; Add To Total Surface
    (set `local.CurrBase` _array_element)
    (bind (_returnvalue_x_3 _returnvalue_y_3) (`KismetMathLibrary.BreakVector` (`SceneComponent.K2_GetComponentScale` (`/Game/Blueprints/BaseSurface.Cube` _array_element))))
    (set `local.Total Surface` (+ (* _returnvalue_x_3 _returnvalue_y_3) (`local.Total Surface`)))
    ; Iterate Through Overlapping Grounds
    (for _array_element_2 (`self.GetOverlappingActors` (`local.CurrBase`) "/Game/Blueprints/GroundSurface.GroundSurface_C")
      (bind _output_get (set `local.CurrGround` _array_element_2))
      (bind _cube_2 (`/Game/Blueprints/GroundSurface.Cube` _output_get))
      (bind (_returnvalue_x_4 _returnvalue_y_4) (`KismetMathLibrary.BreakVector` (`SceneComponent.K2_GetComponentLocation` _cube_2)))
      (bind (_returnvalue_x_5 _returnvalue_y_5) (`KismetMathLibrary.BreakVector` (* (`SceneComponent.K2_GetComponentScale` _cube_2) 0.5)))
      (bind _returnvalue_3 (- _returnvalue_x_4 _returnvalue_x_5))
      ; I'm So Sorry
      (if (> _returnvalue_3 _returnvalue)
        (set `local.CurrWidth` (- _returnvalue_3 _returnvalue))
        (else
          (set `local.CurrWidth` (- (- _returnvalue_x _returnvalue_x_2) (+ _returnvalue_x_4 _returnvalue_x_5)))))
      (bind _returnvalue_4 (- _returnvalue_y_4 _returnvalue_y_5))
      (if (> _returnvalue_4 _returnvalue_2)
        (set `local.CurrHeight` (- _returnvalue_4 _returnvalue_2))
        (else
          (set `local.CurrHeight` (- (- _returnvalue_y _returnvalue_y_2) (+ _returnvalue_y_5 _returnvalue_y_4)))))
      (set `local.Covered Surface` (+ (* (`local.CurrHeight`) (`local.CurrWidth`)) (`local.Covered Surface`)))))
  (return (* (/ (`local.Covered Surface`) (`local.Total Surface`)) 100.0)))

(fn `TryToSnap`
  (params (Node :type "/Game/Blueprints/SnapNode Object Reference"))
  (returns (Succesful :type Boolean))
  (locals (Sphere :type "StaticMeshComponent Object Reference") (`Other Node` :type "/Game/Blueprints/SnapNode Object Reference") (`This Node` :type "/Game/Blueprints/SnapNode Object Reference"))
  (bind _sphere (`/Game/Blueprints/SnapNode.Sphere` Node))
  (bind _returnvalue (`SceneComponent.K2_GetComponentLocation` _sphere))
  ; Search for Snap Nodes in Range
  (set `local.This Node` Node)
  (set `local.Sphere` _sphere)
  (bind _outhits (`KismetSystemLibrary.SphereTraceMulti` _returnvalue _returnvalue (`self.Snap Distance`) "TraceTypeQuery4" false (`self.SnapNodes`)))
  (if (not (`KismetArrayLibrary.Array_IsEmpty` _outhits))
    (for _array_element _outhits
      (bind _assnap_node (cast `/Game/Blueprints/SnapNode` (`.HitActor` (`GameplayStatics.BreakHitResult` _array_element))))
      (bind _output_get (set `local.Other Node` _assnap_node))
      (bind _return (`self.Check Snap Legality` (`local.This Node`) _output_get))
      (if _return
        ; Teleport to Detected Snap Node
        (`self.K2_TeleportTo` (+ (`SceneComponent.K2_GetComponentLocation` (`/Game/Blueprints/SnapNode.Sphere` (`local.Other Node`))) (- (`SceneComponent.K2_GetComponentLocation` (`self.DefaultSceneRoot`)) (`SceneComponent.K2_GetComponentLocation` (`local.Sphere`)))) (`self.Rotation`))
        (return true))))
  (return false))

(fn `UserConstructionScript`)