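; Preview actor that renders a rotating placeable structure into a render target panel through a scene capture.
; On BeginPlay it moves below the origin, applies the Placeable's mesh and materials, and targets the center panel.
; The capture shows only that mesh, with its camera placed at the Placeable's coordinates and aimed at it.
; The mesh yaws every tick regardless of panel, and functions can retarget or clear the capture output.
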(event `self.ReceiveBeginPlay`
  (bind _placeable (`self.Placeable`))
  ; BeginPlay
  (`self.K2_TeleportTo` (0.0 0.0 -500.0))
  (`self.SetStructure` (`/Game/Blueprints/Primary_Placeable.Mesh` _placeable) (`/Game/Blueprints/Primary_Placeable.Materials` _placeable) (`/Game/Blueprints/Primary_Placeable.CameraCoords` _placeable))
  (`self.SetTargetPanel` "/Game/UI/CenterPanel.CenterPanel"))

(event `self.ReceiveTick`
  (params (DeltaSeconds :type "Float (single-precision)"))
  ; Rotate if in Center Panel
  (if true
    (`SceneComponent.K2_AddWorldRotation` (`self.Mesh`) (`KismetMathLibrary.MakeRotator` 0.0 0.0 (* DeltaSeconds 35.0)) false false)))

(fn `NullTargetPanel`
  (set `SceneCaptureComponent2D.TextureTarget` null (`self.SceneCaptureComponent2D`) :!pinned true) ; Sets to null, this is empty on purpose
)

(fn `SetStructure`
  (params (Mesh :type "StaticMesh Object Reference") (Material :type "Array of Material Object Reference") (CamCoords :type "Vector Structure"))
  (`StaticMeshComponent.SetStaticMesh` (`self.Mesh`) Mesh)
  (for (_array_element _array_index) Material
    (`PrimitiveComponent.SetMaterial` (`self.Mesh`) _array_index _array_element))
  (`SceneCaptureComponent.ShowOnlyComponent` (`self.SceneCaptureComponent2D`) (`self.Mesh`))
  (`SceneComponent.K2_SetRelativeLocation` (`self.SceneCaptureComponent2D`) CamCoords false false)
  (`SceneComponent.K2_SetWorldRotation` (`self.SceneCaptureComponent2D`) (`KismetMathLibrary.FindLookAtRotation` (`SceneComponent.K2_GetComponentLocation` (`self.SceneCaptureComponent2D`)) (`SceneComponent.K2_GetComponentLocation` (`self.Mesh`))) false false))

(fn `SetTargetPanel`
  (params (TargetPanel :type "TextureRenderTarget2D Object Reference"))
  (set `SceneCaptureComponent2D.TextureTarget` TargetPanel (`self.SceneCaptureComponent2D`)))

(fn `UserConstructionScript`)